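; Game mode Blueprint for the flower growing game that drives the title, gameplay and game over screens.
; BeginPlay caches BP_FlowerHUD and shows the start menu, while StartGame and GameOver swap widgets and start or stop game systems.
; Tick pushes player stats and distance-based progress to the BP_GameStatus widget, with HP feeding UpdateEnergy and energy feeding UpdateHealth.
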(event EventBeginPlay
  ;[1 1 1] Title menu at start
  (bind _asbp_flower_hud (Utilities|Casting|CastToBP_FlowerHUD (HUD|GetHUD (Game|GetPlayerController 0)))
    (:then
      (Variables|Default|SetAs%20BP%20Flower%20HUD _asbp_flower_hud)
      (Class|FlowerGameHUD|ShowWidget _asbp_flower_hud "Wid_StartGame"))
    (:CastFailed
      (Development|PrintString "failed to detect hud"))))

(event EventTick
  (params (DeltaSeconds :type Float%20%28single-precision%29))
  ;[1 1 1] Status UI update
  (bind _asbp_game_status (Utilities|Casting|CastToBP_GameStatus (Variables|Default|GetBP_statuswidget)))
  (bind _returnvalue (Class|FlowerCellarGameMode|GetPlayerEnergy))
  (bind _returnvalue_2 (Class|FlowerCellarGameMode|GetPlayerResourceRatio))
  (bind _returnvalue_3 (Class|FlowerCellarGameMode|GetCurrentDistance))
  (bind _returnvalue_4 (Class|FlowerCellarGameMode|GetPlayerHP))
  (Class|GameStatusWidget|UpdateEnergy _asbp_game_status _returnvalue_4)
  (Class|GameStatusWidget|UpdateHealth _asbp_game_status _returnvalue)
  (Class|GameStatusWidget|UpdateProgress _asbp_game_status (- 1.0 (/ _returnvalue_3 (Variables|Default|GetTotalDistance))))
  (Class|GameStatusWidget|UpdateResource _asbp_game_status _returnvalue_2))

(event EventStartGame
  ;[1 1 1] Swapping out UI on start and other game modes
  (Class|FlowerGameHUD|HideWidget (stale EventBeginPlay _asbp_flower_hud))
  (bind _returnvalue (Class|FlowerGameHUD|ShowWidget (stale EventBeginPlay _asbp_flower_hud) "Wid_Gameplay" 3))
  (Variables|Default|SetBP_statuswidget _returnvalue)
  (Class|FlowerCellarGameMode|StartSystems))

(event EventGameOver
  ;[1 1 1] Swapping out UI on start and other game modes
  (Class|FlowerGameHUD|HideWidget (stale EventBeginPlay _asbp_flower_hud))
  (Class|FlowerGameHUD|ShowWidget (stale EventBeginPlay _asbp_flower_hud) "Wid_Gameover" 3)
  (Class|FlowerCellarGameMode|StopSystems))

(fn ConstructionScript)